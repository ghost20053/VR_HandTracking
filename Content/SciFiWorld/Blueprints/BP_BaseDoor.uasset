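; Base sci-fi sliding double door that opens automatically on trigger box overlap and closes after a delay, unless locked.
; Box overlap events set open and close request flags, which Tick consumes to start a move and play the matching sound.
; Tick then lerps the two panels along local Y in mirrored directions, handling new requests only once the current move finishes.
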(event `self.ReceiveTick`
  (params (DeltaSeconds :type "Float (single-precision)"))
  (bind _returnvalue (`KismetMathLibrary.MakeVector` 0.0))
  (bind _opened (`self.Opened`))
  (bind _returnvalue_2 (`KismetMathLibrary.MakeVector` 0.0 (`self.MoveDistance`)))
  (bind _returnvalue_3 (`KismetMathLibrary.VLerp` (`KismetMathLibrary.SelectVector` _returnvalue _returnvalue_2 _opened) (`KismetMathLibrary.SelectVector` _returnvalue_2 _returnvalue _opened) (`self.DistanceLerp`)))
  ;[1 1 1] Move doors to current destination
  (if (`self.Moving`)
    (bind _output_get (set `self.DistanceLerp` (+ (`self.DistanceLerp`) (* DeltaSeconds (`self.Speed`)))))
    (`/Engine/EditorBlueprintResources/StandardMacros.CompareFloat` _output_get 1.0
      (:`>`
        (set `self.DistanceLerp` 1.0)
        (set `self.Moving` false))
      (:`<`
        _))
    (if (`KismetSystemLibrary.IsValid` (`self.DoorL`))
      (`SceneComponent.K2_SetRelativeLocation` (`self.DoorL`) _returnvalue_3 false false))
    (if (`KismetSystemLibrary.IsValid` (`self.DoorR`))
      (`SceneComponent.K2_SetRelativeLocation` (`self.DoorR`) (* _returnvalue_3 -1.0) false false))
    (else
      ;[1 1 1] Open/Close states
      (if (`self.NeedClose`)
        (bind _output_get_2 (set `self.CloseTimer` (+ (`self.CloseTimer`) (`GameplayStatics.GetWorldDeltaSeconds`))))
        (`/Engine/EditorBlueprintResources/StandardMacros.CompareFloat` _output_get_2 (`self.CloseDelay`)
          (:`>`
            (set `self.NeedClose` false)
            (set `self.Moving` true)
            (set `self.Opened` false)
            (set `self.DistanceLerp` 0.0)
            (set `self.CloseTimer` 0.0)
            (`AudioComponent.Play` (`self.AudioClose`) 0.0)))
        (elif (`self.NeedOpen`)
          (set `self.NeedOpen` false)
          (set `self.Moving` true)
          (set `self.Opened` true)
          (set `self.DistanceLerp` 0.0)
          (`AudioComponent.Play` (`self.AudioOpen`) 0.0))))))

(event `self.Box.OnComponentBeginOverlap`
  (params (OverlappedComponent :type "PrimitiveComponent Object Reference") (OtherActor :type "Actor Object Reference") (OtherComp :type "PrimitiveComponent Object Reference") (OtherBodyIndex :type Integer) (bFromSweep :type Boolean) (SweepResult :type "HitResult Structure (by ref)"))
  (if (and (not (`self.Locked`)) (not (`self.NeedOpen`)))
    (set `self.NeedOpen` true)
    (set `self.NeedClose` false)))

(event `self.Box.OnComponentEndOverlap`
  (params (OverlappedComponent :type "PrimitiveComponent Object Reference") (OtherActor :type "Actor Object Reference") (OtherComp :type "PrimitiveComponent Object Reference") (OtherBodyIndex :type Integer))
  (if (not (`self.Locked`))
    (set `self.NeedClose` true)))

(fn `UserConstructionScript`)