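; Test Blueprint for loading Mixed Reality Utility Kit (MRUK) spatial scene data from the device, reporting progress through on-screen prints.
; BeginPlay binds to the scene-loaded event, requests a delayed load, then prints the load status.
; The callback confirms a valid room, or on failure makes one delayed async load attempt.
; An alternative XR-readiness poll with recursive retry loading exists but is never started.
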(event `self.ReceiveBeginPlay`
  (bind _returnvalue (subsystem `MRUKSubsystem`))
  (add `MRUKSubsystem.OnSceneLoaded` (subsystem `MRUKSubsystem`) (delegate `SceneStatus`))
  (`KismetSystemLibrary.Delay` 1.0)
  (`MRUKSubsystem.LoadSceneFromDevice` _returnvalue "V1")
  (`KismetSystemLibrary.Delay` 3.0)
  (`KismetSystemLibrary.PrintString` (`|GetEnumeratorNameAsString` (`MRUKSubsystem.SceneLoadStatus` _returnvalue)) true true (struct :`G` 0.66 :`B` 1.0 :`A` 1.0) 10.0))

(event `SceneStatus`
  (params (Success :type Boolean))
  (if Success
    (`KismetSystemLibrary.PrintString` (`|GetEnumeratorNameAsString` (`MRUKSubsystem.SceneLoadStatus` (subsystem `MRUKSubsystem`))) true true (struct :`G` 0.66 :`B` 1.0 :`A` 1.0) 10.0)
    (`/Engine/EditorBlueprintResources/StandardMacros.IsValid` (`MRUKSubsystem.GetCurrentRoom` (subsystem `MRUKSubsystem`))
      (:`Is Valid`
        (`KismetSystemLibrary.PrintString` "Valid Room" true true (struct :`G` 0.66 :`B` 1.0 :`A` 1.0) 10.0)))
    (else
      (`KismetSystemLibrary.PrintString` "SCENE FAILED" true true (struct :`G` 0.66 :`B` 1.0 :`A` 1.0) 10.0)
      (`KismetSystemLibrary.Delay` 2.0)
      (`MRUKLoadFromDevice.LoadSceneFromDeviceAsync` "V1"
        (:`Success`
          (`KismetSystemLibrary.PrintString` "SPATIAL DATA LOADED" true true (struct :`G` 0.66 :`B` 1.0 :`A` 1.0) 10.0))
        (:`Failure`
          (`KismetSystemLibrary.PrintString` "SPATIAL DATA FAILED" true true (struct :`G` 0.66 :`B` 1.0 :`A` 1.0) 10.0))))))

(event `CheckXRready`
  (if (`HeadMountedDisplayFunctionLibrary.IsHeadMountedDisplayEnabled`)
    (`KismetSystemLibrary.PrintString` "XR Ready" true true (struct :`G` 0.66 :`B` 1.0 :`A` 1.0) 10.0)
    (`KismetSystemLibrary.Delay` 1.0)
    (`MRUKLoadFromDevice.LoadSceneFromDeviceAsync` "V1"
      (:`Success`
        (`KismetSystemLibrary.PrintString` "SPATIAL DATA LOADED" true true (struct :`G` 0.66 :`B` 1.0 :`A` 1.0) 10.0))
      (:`Failure`
        (`KismetSystemLibrary.PrintString` "LOAD FAILED - RETRYING" true true (struct :`G` 0.66 :`B` 1.0 :`A` 1.0) 10.0)
        (`self.TryLoad Scene`)))
    (else
      (`KismetSystemLibrary.Delay` 1.0)
      (`self.CheckXRready`))))

(event `TryLoad Scene`
  (`MRUKLoadFromDevice.LoadSceneFromDeviceAsync` "V1"
    (:`Success`
      (`KismetSystemLibrary.PrintString` "SPATIAL DATA LOADED" true true (struct :`G` 0.66 :`B` 1.0 :`A` 1.0) 10.0))
    (:`Failure`
      (`KismetSystemLibrary.PrintString` "LOAD FAILED - RETRYING" true true (struct :`G` 0.66 :`B` 1.0 :`A` 1.0) 10.0)
      (`KismetSystemLibrary.Delay` 2.0)
      (`self.TryLoad Scene`))))

(fn `UserConstructionScript`)