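; BP_Door is an interactable door in the hand tracking interactions folder that swings open or closed each time it receives BeginInteract.
; The event toggles IsOpen and plays or reverses the TL_OpenDoor timeline.
; Timeline updates lerp the yaw of DoorPivot between ClosedAngle and OpenAngle as a relative rotation.
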(event `/Game/HandTracking/BPI_Interactable.Begin_Interact`
  (if (`self.IsOpen`)
    (set `self.IsOpen` false)
    (bind (_direction _newtrack_0) (`Timeline|TL_OpenDoor` :!via `Reverse` :!label _label)
      (:`Update`
        (`SceneComponent.K2_SetRelativeRotation` (`self.DoorPivot`) (`KismetMathLibrary.MakeRotator` 0.0 0.0 (`KismetMathLibrary.Lerp` (`self.ClosedAngle`) (`self.OpenAngle`) _newtrack_0)) false false)))
    (else
      (set `self.IsOpen` true)
      (goto _label))))

(fn `UserConstructionScript`)