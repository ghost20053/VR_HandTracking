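; BP_QRTrackingManager turns Meta MRUK QR code detections into transform updates for a tracked cube.
; On BeginPlay it enables QR-only trackable tracking and, on success, binds to the subsystem's added, updated and removed events.
; Added and updated trackables pass payload and transform to HandleQRUpdate, which matches the payload and calls UpdateFromQR on Cube01.
; Only Cube 01 face A is mapped, and removal is ignored.
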(event `Handle QR Update`
  (params (Payload :type String) (QRTransform :type "Transform Structure"))
  (switch `string` Payload
    (:`CUBE_01_FACE_A`
      (`/Game/HandTracking/QR_Code/BP_QRCube.Update From QR` (`self.Cube01`) QRTransform "CUBE_01_FACE_A"))))

(event `self.ReceiveBeginPlay`
  (bind _returnvalue (subsystem `MRUKSubsystem`))
  (`MRUKConfigureTrackables.ConfigureTrackablesAsync` (make `MRUKTrackerConfiguration` false true)
    (:`Success`
      (`KismetSystemLibrary.PrintString` "QR TRACKING CONFIGURATION successful")
      (add `MRUKSubsystem.OnTrackableAdded` _returnvalue (delegate `OnTrackableAdded_Event`))
      (add `MRUKSubsystem.OnTrackableUpdated` _returnvalue (delegate `OnTrackableUpdated_Event`))
      (add `MRUKSubsystem.OnTrackableRemoved` _returnvalue (delegate `OnTrackableRemoved_Event`)))
    (:`Failure`
      (`KismetSystemLibrary.PrintString` "QR TRACKING CONFIGURATION FAILED"))))

(event `OnTrackableAdded_Event`
  (params (Trackable :type "MRUKTrackable Object Reference"))
  (`self.Handle QR Update` (`MRUKTrackable.MarkerPayloadString` Trackable) (`self.GetTransform` Trackable)))

(event `OnTrackableUpdated_Event`
  (params (Trackable :type "MRUKTrackable Object Reference"))
  (`self.Handle QR Update` (`MRUKTrackable.MarkerPayloadString` Trackable) (`self.GetTransform` Trackable)))

(event `OnTrackableRemoved_Event`
  (params (Trackable :type "MRUKTrackable Object Reference")))

(fn `UserConstructionScript`)