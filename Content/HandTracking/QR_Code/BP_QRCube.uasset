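; BP_QRCube is a hand-tracking cube actor that can be grabbed and placed at a QR code's pose.
; UpdateFromQR snaps the actor to the supplied transform; its Face input is unused.
; IsdkGrabbable interactor changes switch off physics while interactors are present, restoring gravity and simulation after a brief delay once none remain.
; Select and unselect events track an active grab count, used only for debug printing.
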(event `self.ReceiveBeginPlay`
  (`KismetSystemLibrary.PrintString` (`KismetStringLibrary.Conv_VectorToString` (* (`.BoxExtent` (`self.GetActorBounds` false)) 2.0)) true true (struct :`G` 0.66 :`B` 1.0 :`A` 1.0) 10.0))

(event `self.IsdkGrabbable.StateChangedDelegate`
  (params (InteractableState :type "IsdkInteractableStateEvent Structure (by ref)")))

(event `self.IsdkGrabbable.InteractorCountChangedDelegate`
  (params (Sender :type "IsdkSceneInteractableComponent Object Reference") (NewCount :type Integer))
  (bind _cube (`self.Cube`))
  (if (== NewCount 0)
    (`KismetSystemLibrary.Delay` 0.01)
    (`PrimitiveComponent.SetEnableGravity` _cube true)
    (`PrimitiveComponent.SetSimulatePhysics` _cube true)
    (else
      (`PrimitiveComponent.SetSimulatePhysics` (`self.Cube`) false))))

(event `self.IsdkGrabbable.InteractionPointerEvent`
  (params (PointerEvent :type "IsdkInteractionPointerEvent Structure (by ref)"))
  (bind _activegrabcount (`self.ActiveGrabCount`))
  (switch `EIsdkPointerEventType` PointerEvent_Type
    (:`Select`
      (bind _output_get (set `self.ActiveGrabCount` (+ _activegrabcount 1))))
    (:`Unselect`
      (bind _output_get_2 (set `self.ActiveGrabCount` (`KismetMathLibrary.Max` (- _activegrabcount 1))))
      (`KismetSystemLibrary.PrintString` (`KismetStringLibrary.Conv_IntToString` _output_get_2) true true (struct :`G` 0.66 :`B` 1.0 :`A` 1.0) 10.0)
      (if (== _output_get_2 0)
        _))))

(event `Update From QR`
  (params (QRTransform :type "Transform Structure") (Face :type String))
  (`self.K2_SetActorTransform` QRTransform))

(fn `UserConstructionScript`)