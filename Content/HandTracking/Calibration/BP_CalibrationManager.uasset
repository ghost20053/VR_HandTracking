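; Calibration manager that aligns the virtual world to the player's hands at a table, then transitions from Meta passthrough into VR.
; Tick runs a hold timer while both pawn calibration spheres stay level, suitably spaced and still, driving the calibration UI.
; On completion it translates BP_CalibrationRoot so its hand anchor meets the hands' midpoint, fades passthrough, spawns props and animates a material-collection world scan.
; Hand trigger overlaps only set unused flags and print.
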(event `self.ReceiveBeginPlay`
  (bind _returnvalue (subsystem `OculusXRPassthroughSubsystem`))
  (`/Engine/EditorBlueprintResources/StandardMacros.IsValid` _returnvalue
    (:`Is Valid`
      (bind _returnvalue_2 (`OculusXRPassthroughSubsystem.InitializePersistentPassthrough` :`self` _returnvalue))
      (set `self.PersistentPassthrough` _returnvalue_2)
      (`self.EnableInput` (`GameplayStatics.GetPlayerController` 0))
      (bind _asbp_isdkmeta_pawn (cast `/Game/HandTracking/BP_ISDKMeta_Pawn` (`GameplayStatics.GetPlayerPawn` 0)))
      (set `self.Left Calibration Sphere Ref` (`/Game/HandTracking/BP_ISDKMeta_Pawn.LeftCalibrationSphere` _asbp_isdkmeta_pawn))
      (set `self.Right Calibration Sphere Ref` (`/Game/HandTracking/BP_ISDKMeta_Pawn.RightCalibrationSphere` _asbp_isdkmeta_pawn))
      (bind _returnvalue_3 (`GameplayStatics.GetActorOfClass` "/Game/HandTracking/Calibration/BP_CalibrationRoot.BP_CalibrationRoot_C"))
      (bind _output_get (set `self.CalibrationRoot` _returnvalue_3))
      (`/Game/HandTracking/Calibration/BP_CalibrationRoot.SetVirtualWorldVisible` _output_get false)
      (`self.HandAlingment`)
      (bind _returnvalue_4 (`GameplayStatics.GetActorOfClass` "/Game/HandTracking/Table/BP_UI.BP_UI_C"))
      (bind _output_get_2 (set `self.CalibrationUIActor` _returnvalue_4))
      (bind _aswbp_calibration_ui (cast `/Game/HandTracking/Calibration/WBP_CalibrationUI` (`WidgetComponent.GetUserWidgetObject` (`/Game/HandTracking/Table/BP_UI.Widget` _output_get_2))))
      (bind _output_get_3 (set `self.CalibrationUI` _aswbp_calibration_ui))
      (`/Game/HandTracking/Calibration/WBP_CalibrationUI.SetWaitingState` _output_get_3)
      (`KismetSystemLibrary.Delay` 4.0)
      (set `self.CanStartCalibration` true))))

(event `self.ReceiveTick`
  (params (DeltaSeconds :type "Float (single-precision)"))
  (bind _calibrationui (`self.CalibrationUI`))
  (bind _handdistance (`self.HandDistance`))
  (bind _left_calibration_sphere_ref (`self.Left Calibration Sphere Ref`))
  (bind _right_calibration_sphere_ref (`self.Right Calibration Sphere Ref`))
  (bind (_returnvalue_x _returnvalue_y _returnvalue_z) (`KismetMathLibrary.BreakVector` (`SceneComponent.K2_GetComponentLocation` _left_calibration_sphere_ref)))
  (bind (_returnvalue_x_2 _returnvalue_y_2 _returnvalue_z_2) (`KismetMathLibrary.BreakVector` (`SceneComponent.K2_GetComponentLocation` _right_calibration_sphere_ref)))
  (set `self.HandDistance` (`KismetMathLibrary.Vector_Distance` (`SceneComponent.K2_GetComponentLocation` (`self.Left Calibration Sphere Ref`)) (`SceneComponent.K2_GetComponentLocation` (`self.Right Calibration Sphere Ref`))))
  (if (and (and (not (`self.CalibrationComplete`)) (not (`self.IsTransitioning`))) (`self.CanStartCalibration`))
    (if (not (`self.HasPositionedManager`))
      (`self.PositionManagerAtHands`)
      (set `self.HasPositionedManager` true))
    (if (and (and (<= (`KismetMathLibrary.Abs` (- _returnvalue_z _returnvalue_z_2)) (`self.HandHeightTolerance`)) (and (>= _handdistance 20.0) (<= _handdistance 40.0))) (and (<= (`KismetMathLibrary.Vector_Distance` (`SceneComponent.K2_GetComponentLocation` _left_calibration_sphere_ref) (`self.PreviousLeftHandLocation`)) (`self.MaxHandMovement`)) (<= (`KismetMathLibrary.Vector_Distance` (`SceneComponent.K2_GetComponentLocation` _right_calibration_sphere_ref) (`self.PreviousRightHandLocation`)) (`self.MaxHandMovement`))))
      (`/Game/HandTracking/Calibration/WBP_CalibrationUI.SetCalibratingState` (`self.CalibrationUI`))
      (bind _output_get (set `self.CurrentHoldTimer` (+ (`self.CurrentHoldTimer`) (`GameplayStatics.GetWorldDeltaSeconds`))))
      (`/Game/HandTracking/Calibration/WBP_CalibrationUI.UpdateCalibrationProgress` (`self.CalibrationUI`) (`KismetMathLibrary.FClamp` (/ _output_get 10.0)))
      (if (>= (`self.CurrentHoldTimer`) 10.0)
        (set `self.CurrentHoldTimer` 2.0)
        (`/Game/HandTracking/Calibration/WBP_CalibrationUI.SetCompleteState` (`self.CalibrationUI`))
        (`self.StartCalibration`)
        (else
          (set `self.PreviousLeftHandLocation` (`SceneComponent.K2_GetComponentLocation` (`self.Left Calibration Sphere Ref`)) :!label _label)
          (set `self.PreviousRightHandLocation` (`SceneComponent.K2_GetComponentLocation` (`self.Right Calibration Sphere Ref`)))))
      (else
        (bind _output_get_2 (set `self.CurrentHoldTimer` 0.0))
        (`/Game/HandTracking/Calibration/WBP_CalibrationUI.UpdateCalibrationProgress` _calibrationui _output_get_2)
        (`/Game/HandTracking/Calibration/WBP_CalibrationUI.SetWaitingState` _calibrationui)
        (goto _label)))))

(event `self.LeftTrigger.OnComponentBeginOverlap`
  (params (OverlappedComponent :type "PrimitiveComponent Object Reference") (OtherActor :type "Actor Object Reference") (OtherComp :type "PrimitiveComponent Object Reference") (OtherBodyIndex :type Integer) (bFromSweep :type Boolean) (SweepResult :type "HitResult Structure (by ref)"))
  (if (`ActorComponent.ComponentHasTag` OtherComp "LeftCalibration")
    (bind _output_get (set `self.LeftHandInside` true))
    (`KismetSystemLibrary.PrintString` "Left Hand Entered" _output_get _output_get (struct :`G` 0.66 :`B` 1.0 :`A` 1.0) 10.0)))

(event `StartCalibration`
  (bind _calibrationroot (`self.CalibrationRoot`))
  (bind _output_get (set `self.HandsMidPoint` (/ (+ (`SceneComponent.K2_GetComponentLocation` (`self.Left Calibration Sphere Ref`)) (`SceneComponent.K2_GetComponentLocation` (`self.Right Calibration Sphere Ref`))) 2.0)))
  (`self.K2_SetActorLocation` (`self.CalibrationRoot`) (+ (`self.K2_GetActorLocation` _calibrationroot) (- _output_get (`SceneComponent.K2_GetComponentLocation` (`/Game/HandTracking/Calibration/BP_CalibrationRoot.HandResetAnchor` _calibrationroot)))) false false)
  (set `self.IsTransitioning` true)
  (`PrimitiveComponent.SetCollisionEnabled` (`self.LeftTrigger`) "NoCollision")
  (`PrimitiveComponent.SetCollisionEnabled` (`self.RightTrigger`) "NoCollision")
  (`SceneComponent.SetVisibility` (`self.LeftGhostHand`) false false)
  (`SceneComponent.SetVisibility` (`self.RightGhostHand`) false false)
  (`SceneComponent.SetVisibility` (`self.LeftHandSkeletalMesh`) false false)
  (`SceneComponent.SetVisibility` (`self.RightHandSkeletalMesh`) false false)
  (`KismetSystemLibrary.PrintString` "Table Calibration Complete" true true (struct :`G` 0.66 :`B` 1.0 :`A` 1.0) 10.0)
  (bind (_direction _transition) (`Timeline|TransitionTimeline` :!via `PlayFromStart`)
    (:`Update`
      (bind _returnvalue (- 1.0 _transition))
      (`OculusXRPassthroughLayerBase.SetTextureOpacity` (`OculusXRPersistentPassthroughInstance.GetShape` (`self.PersistentPassthrough`)) _returnvalue)
      (`WidgetComponent.SetTintColorAndOpacity` (`/Game/HandTracking/Table/BP_UI.Widget` (`self.CalibrationUIActor`)) (`KismetMathLibrary.Conv_DoubleToLinearColor` _returnvalue)))
    (:`Finished`
      (`|ExecutionSequence`
        (:`then_0`
          (`OculusXRPersistentPassthroughInstance.SetVisible` (`self.PersistentPassthrough`) false)
          (`/Game/HandTracking/Calibration/BP_CalibrationRoot.SetVirtualWorldVisible` (`self.CalibrationRoot`) true)
          (`/Game/HandTracking/Calibration/BP_CalibrationRoot.SpawnProps` (`self.CalibrationRoot`))
          (`self.K2_DestroyActor` (`self.CalibrationUIActor`))
          (set `self.IsTransitioning` false)
          (set `self.CalibrationComplete` true)
          (`self.SetActorTickEnabled` false))
        (:`then_1`
          (bind _outactors (`GameplayStatics.GetAllActorsWithTag` "VirtualEnvironment"))
          (for _array_element _outactors
            (`self.SetActorHiddenInGame` _array_element false))
          (bind (_direction_2 _scanamount) (`Timeline|TL_WorldScan` :!via `PlayFromStart`)
            (:`Update`
              (`KismetMaterialLibrary.SetScalarParameterValue` "/Game/HandTracking/Material/MPC_VRTransition.MPC_VRTransition" "ScanAmount" _scanamount)
              (`KismetSystemLibrary.PrintString` (`KismetStringLibrary.Conv_DoubleToString` _scanamount)))))))))

(event `self.LeftTrigger.OnComponentEndOverlap`
  (params (OverlappedComponent :type "PrimitiveComponent Object Reference") (OtherActor :type "Actor Object Reference") (OtherComp :type "PrimitiveComponent Object Reference") (OtherBodyIndex :type Integer))
  (if (`ActorComponent.ComponentHasTag` OtherComp "LeftCalibration")
    (bind _output_get (set `self.LeftHandInside` false))
    (`KismetSystemLibrary.PrintString` "Left Hand Left" _output_get _output_get (struct :`G` 0.66 :`B` 1.0 :`A` 1.0) 10.0)))

(event `PositionManagerAtHands`
  (`self.K2_SetActorLocation` (+ (/ (+ (`SceneComponent.K2_GetComponentLocation` (`self.Left Calibration Sphere Ref`)) (`SceneComponent.K2_GetComponentLocation` (`self.Right Calibration Sphere Ref`))) 2.0) (0.0 0.0 2.0))))

(event `self.RightTrigger.OnComponentBeginOverlap`
  (params (OverlappedComponent :type "PrimitiveComponent Object Reference") (OtherActor :type "Actor Object Reference") (OtherComp :type "PrimitiveComponent Object Reference") (OtherBodyIndex :type Integer) (bFromSweep :type Boolean) (SweepResult :type "HitResult Structure (by ref)"))
  (if (`ActorComponent.ComponentHasTag` OtherComp "RightCalibration")
    (bind _output_get (set `self.RightHandInside` true))
    (`KismetSystemLibrary.PrintString` "Right Hand Entered" _output_get _output_get (struct :`R` 1.0 :`B` 0.051269 :`A` 1.0) 10.0)))

(event `self.RightTrigger.OnComponentEndOverlap`
  (params (OverlappedComponent :type "PrimitiveComponent Object Reference") (OtherActor :type "Actor Object Reference") (OtherComp :type "PrimitiveComponent Object Reference") (OtherBodyIndex :type Integer))
  (if (`ActorComponent.ComponentHasTag` OtherComp "RightCalibration")
    (bind _output_get (set `self.RightHandInside` false))
    (`KismetSystemLibrary.PrintString` "Right Hand Left" _output_get _output_get (struct :`R` 1.0 :`B` 0.051269 :`A` 1.0) 10.0)))

(event `HandAlingment`
  (bind _asbp_isdkmeta_pawn (cast `/Game/HandTracking/BP_ISDKMeta_Pawn` (`GameplayStatics.GetPlayerPawn` 0)))
  (bind _vrcamera (`/Game/HandTracking/BP_ISDKMeta_Pawn.VRCamera` _asbp_isdkmeta_pawn))
  (bind _returnvalue (`KismetMathLibrary.MakeRotator` 0.0 0.0 (.yaw (`SceneComponent.K2_GetComponentRotation` _vrcamera))))
  (`self.K2_SetActorLocation` (+ (+ (`SceneComponent.K2_GetComponentLocation` _vrcamera) (* (`KismetMathLibrary.GetForwardVector` _returnvalue) (`self.CalibrationDistance`))) (`KismetMathLibrary.MakeVector` 0.0 0.0 (`self.ChestHeightOffset`))))
  (`self.K2_SetActorRotation` _returnvalue))

(fn `UserConstructionScript`)