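; VR hand-tracking Blueprint that turns Oculus thumb pinches into right-hand grabbing and left-hand force pull and push.
; A right pinch sphere-traces for "Grabbable" actors and attaches the hit to the controller, restoring physics on release.
; A left pinch pulls "ForceObject" actors with distance-scaled velocity, attaches them within catch range, then launches them forward and slightly upward on release.
; IsRightHandClosed is an unfinished bone-location check.
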(event `self.ReceiveBeginPlay`
  (`HeadMountedDisplayFunctionLibrary.SetTrackingOrigin` "LocalFloor")
  (`OculusXRInputFunctionLibrary.SetControllerDrivenHandPoses` "Natural"))

(event `InputAxisKey|OculusHand_Right_ThumbPinchStrength`
  (params (AxisValue :type "Float (single-precision)"))
  (bind _grabbedobject (`self.GrabbedObject`))
  (bind _motioncontroller_right (`self.MotionController_Right`))
  (bind _returnvalue (`self.GetComponentByClass` _grabbedobject "/Script/Engine.StaticMeshComponent"))
  ; Right Hand Picking Up Object
  (`|ExecutionSequence`
    (:`then_0`
      ;; Grabbing Object
      (if (> AxisValue 0.8)
        (set `self.IsHoldingObject` false)
        (`/Engine/EditorBlueprintResources/StandardMacros.DoOnce` false :!label _label
          (:`Completed`
            (bind _outhit (`KismetSystemLibrary.SphereTraceSingleForObjects` (`SceneComponent.K2_GetComponentLocation` _motioncontroller_right) (* (`SceneComponent.GetForwardVector` _motioncontroller_right) 100.0) (`self.GrabRadius`) (`|MakeArray` "ObjectTypeQuery4" "ObjectTypeQuery2" :!type "EObjectTypeQuery Enum")))
            (bind (_bblockinghit _binitialoverlap _time _distance _location _impactpoint _normal _impactnormal _physmat _hitactor) (`GameplayStatics.BreakHitResult` _outhit))
            (if _bblockinghit
              (if (`self.ActorHasTag` _hitactor "Grabbable")
                (bind _output_get (set `self.GrabbedObject` _hitactor))
                (set `self.IsHoldingObject` true)
                (`PrimitiveComponent.SetSimulatePhysics` (`self.GetComponentByClass` _hitactor "/Script/Engine.StaticMeshComponent") false)
                (`self.K2_AttachToComponent` _output_get (`self.MotionController_Right`) "None" "SnapToTarget" "SnapToTarget" "KeepWorld" false)))))))
    (:`then_1`
      ;; Release Object
      (if (< AxisValue 0.2)
        (bind _output_get_2 (set `self.IsHoldingObject` true))
        (if _output_get_2
          (`/Engine/EditorBlueprintResources/StandardMacros.IsValid` _returnvalue
            (:`Is Valid`
              (`self.K2_DetachFromActor` _grabbedobject "KeepWorld" "KeepWorld" "KeepWorld")
              (`PrimitiveComponent.SetSimulatePhysics` _returnvalue true)
              (set `self.GrabbedObject` null)
              (set `self.IsHoldingObject` false)
              (goto _label :!via `Reset`))))))))

(event `InputAxisKey|OculusHand_Left_ThumbPinchStrength`
  (params (AxisValue :type "Float (single-precision)"))
  (bind _forcetarget (`self.ForceTarget`))
  (bind _motioncontroller_left (`self.MotionController_Left`))
  (bind _motioncontroller_left_2 (`self.MotionController_Left`))
  (bind _returnvalue (`SceneComponent.K2_GetComponentLocation` (`self.MotionController_Left`)))
  (bind _returnvalue_2 (`SceneComponent.K2_GetComponentLocation` _motioncontroller_left_2))
  ; Left Hand Force Pull and Push
  (`|ExecutionSequence`
    (:`then_0`
      ;; Force Pull
      (if (> AxisValue 0.3)
        (set `self.IsForceHolding` false)
        (if (not (`self.IsForceHolding`))
          (bind _outhit (`KismetSystemLibrary.SphereTraceSingleForObjects` _returnvalue_2 (+ _returnvalue_2 (* (`SceneComponent.GetForwardVector` _motioncontroller_left_2) 1500.0)) (`self.ForceRadius`) (`|MakeArray` "ObjectTypeQuery4" "ObjectTypeQuery2" :!type "EObjectTypeQuery Enum")))
          (bind (_bblockinghit _binitialoverlap _time _distance _location _impactpoint _normal _impactnormal _physmat _hitactor) (`GameplayStatics.BreakHitResult` _outhit))
          (if _bblockinghit
            (if (`self.ActorHasTag` _hitactor "ForceObject")
              (bind _returnvalue_3 (`self.K2_GetActorLocation` _hitactor))
              (`PrimitiveComponent.SetPhysicsLinearVelocity` (`self.GetComponentByClass` _hitactor "/Script/Engine.StaticMeshComponent") (* (* (`KismetMathLibrary.FClamp` (/ (`KismetMathLibrary.Vector_Distance` _returnvalue _returnvalue_3) 200.0) 0.2) (`self.ForcePullSpeed`)) (`KismetMathLibrary.Normal` (- _returnvalue _returnvalue_3))) false "None")
              (bind _output_get (set `self.ForceTarget` _hitactor))
              (set `self.ForceTargetMesh` (`self.GetComponentByClass` _output_get "/Script/Engine.StaticMeshComponent"))
              (if (< (`KismetMathLibrary.Vector_Distance` (`SceneComponent.K2_GetComponentLocation` (`self.MotionController_Left`)) (`self.K2_GetActorLocation` (`self.ForceTarget`))) (`self.CatchDistance`))
                (`PrimitiveComponent.SetSimulatePhysics` (`self.ForceTargetMesh`) false)
                (`self.K2_AttachToComponent` (`self.ForceTarget`) (`self.MotionController_Left`) "None" "SnapToTarget" "SnapToTarget" "KeepWorld" false)
                (set `self.IsForceHolding` true)))))))
    (:`then_1`
      ;; Force Push
      (if (< AxisValue 0.2)
        (set `self.IsForceHolding` true)
        (`/Engine/EditorBlueprintResources/StandardMacros.IsValid` _forcetarget
          (:`Is Valid`
            (`self.K2_DetachFromActor` _forcetarget "KeepWorld" "KeepWorld" "KeepWorld")
            (`PrimitiveComponent.SetSimulatePhysics` (`self.ForceTargetMesh`) true)
            (`PrimitiveComponent.AddImpulse` (`self.ForceTargetMesh`) (* (`KismetMathLibrary.Normal` (+ (`SceneComponent.GetForwardVector` _motioncontroller_left) (* (`SceneComponent.GetUpVector` _motioncontroller_left) 0.2))) (`self.ForcePushStrength`)) "None" true)
            (set `self.ForceTarget` null)
            (set `self.ForceTargetMesh` null)
            (set `self.IsForceHolding` false)))))))

(fn `IsRightHandClosed`
  (bind _oculusxrhand_right (`self.OculusXRHand_Right`))
  (`|ExecutionSequence`
    (:`then_0`
      (bind _returnvalue (`PoseableMeshComponent.GetBoneLocationByName` _oculusxrhand_right "WristRoot" "WorldSpace"))
      (`/Engine/EditorBlueprintResources/StandardMacros.IncrementFloat` (`KismetMathLibrary.Conv_BoolToDouble` (< (`KismetMathLibrary.Vector_Distance` _returnvalue) 12.0))))
    (:`then_1`
      (`PoseableMeshComponent.GetBoneLocationByName` _oculusxrhand_right "ThumbTip" "WorldSpace"))
    (:`then_2`
      (`PoseableMeshComponent.GetBoneLocationByName` _oculusxrhand_right "IndexTip" "WorldSpace"))
    (:`then_3`
      (`PoseableMeshComponent.GetBoneLocationByName` _oculusxrhand_right "MiddleTip" "WorldSpace"))
    (:`then_4`
      (`PoseableMeshComponent.GetBoneLocationByName` _oculusxrhand_right "RingTip" "WorldSpace"))
    (:`then_5`
      (`PoseableMeshComponent.GetBoneLocationByName` _oculusxrhand_right "PinkyTip" "WorldSpace"))))

(fn `UserConstructionScript`)