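; Calibration manager that aligns the table setup to the player's tracked hands in a hand-tracking game.
; Left and right triggers detect tagged calibration components, and Tick runs a hold timer while both hands stay inside.
; After two seconds, it translates BP_CalibrationRoot so its HandResetAnchor meets the midpoint of the pawn's calibration spheres, without changing rotation.
; It then spawns the props, disables both triggers and hides the ghost hands.
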(event `self.ReceiveBeginPlay`
  (bind _asbp_isdkmeta_pawn (cast `/Game/HandTracking/BP_ISDKMeta_Pawn` (`GameplayStatics.GetPlayerPawn` 0)))
  (set `self.Left Calibration Sphere Ref` (`/Game/HandTracking/BP_ISDKMeta_Pawn.LeftCalibrationSphere` _asbp_isdkmeta_pawn))
  (set `self.Right Calibration Sphere Ref` (`/Game/HandTracking/BP_ISDKMeta_Pawn.RightCalibrationSphere` _asbp_isdkmeta_pawn))
  (bind _returnvalue (`GameplayStatics.GetActorOfClass` "/Game/HandTracking/Table/BP_CalibrationRoot.BP_CalibrationRoot_C"))
  (set `self.CalibrationRoot` _returnvalue))

(event `self.ReceiveTick`
  (params (DeltaSeconds :type "Float (single-precision)"))
  (if (not (`self.CalibrationComplete`))
    (if (== (and (`self.LeftHandInside`) (`self.RightHandInside`)) true)
      (set `self.CurrentHoldTimer` (+ (`self.CurrentHoldTimer`) (`GameplayStatics.GetWorldDeltaSeconds`)))
      (if (>= (`self.CurrentHoldTimer`) 2.0)
        (set `self.CalibrationComplete` true)
        (set `self.CurrentHoldTimer` 2.0)
        (`self.StartCalibration`))
      (else
        (set `self.CurrentHoldTimer` 0.0)))))

(event `self.LeftTrigger.OnComponentBeginOverlap`
  (params (OverlappedComponent :type "PrimitiveComponent Object Reference") (OtherActor :type "Actor Object Reference") (OtherComp :type "PrimitiveComponent Object Reference") (OtherBodyIndex :type Integer) (bFromSweep :type Boolean) (SweepResult :type "HitResult Structure (by ref)"))
  (if (`ActorComponent.ComponentHasTag` OtherComp "LeftCalibration")
    (bind _output_get (set `self.LeftHandInside` true))
    (`KismetSystemLibrary.PrintString` "Left Hand Entered" _output_get _output_get (struct :`G` 0.66 :`B` 1.0 :`A` 1.0) 10.0)))

(event `self.LeftTrigger.OnComponentEndOverlap`
  (params (OverlappedComponent :type "PrimitiveComponent Object Reference") (OtherActor :type "Actor Object Reference") (OtherComp :type "PrimitiveComponent Object Reference") (OtherBodyIndex :type Integer))
  (if (`ActorComponent.ComponentHasTag` OtherComp "LeftCalibration")
    (bind _output_get (set `self.LeftHandInside` false))
    (`KismetSystemLibrary.PrintString` "Left Hand Left" _output_get _output_get (struct :`G` 0.66 :`B` 1.0 :`A` 1.0) 10.0)))

(event `StartCalibration`
  (bind _calibrationroot (`self.CalibrationRoot`))
  (bind _output_get (set `self.HandsMidPoint` (/ (+ (`SceneComponent.K2_GetComponentLocation` (`self.Left Calibration Sphere Ref`)) (`SceneComponent.K2_GetComponentLocation` (`self.Right Calibration Sphere Ref`))) 2.0)))
  (`self.K2_SetActorLocation` (`self.CalibrationRoot`) (+ (`self.K2_GetActorLocation` _calibrationroot) (- _output_get (`SceneComponent.K2_GetComponentLocation` (`/Game/HandTracking/Table/BP_CalibrationRoot.HandResetAnchor` _calibrationroot)))) false false)
  (`/Game/HandTracking/Table/BP_CalibrationRoot.SpawnProps` (`self.CalibrationRoot`))
  (`PrimitiveComponent.SetCollisionEnabled` (`self.LeftTrigger`) "NoCollision")
  (`PrimitiveComponent.SetCollisionEnabled` (`self.RightTrigger`) "NoCollision")
  (`SceneComponent.SetVisibility` (`self.LeftGhostHand`) false false)
  (`SceneComponent.SetVisibility` (`self.RightGhostHand`) false false)
  (`KismetSystemLibrary.PrintString` "Table Calibration COmplete" true true (struct :`G` 0.66 :`B` 1.0 :`A` 1.0) 10.0))

(event `self.RightTrigger.OnComponentBeginOverlap`
  (params (OverlappedComponent :type "PrimitiveComponent Object Reference") (OtherActor :type "Actor Object Reference") (OtherComp :type "PrimitiveComponent Object Reference") (OtherBodyIndex :type Integer) (bFromSweep :type Boolean) (SweepResult :type "HitResult Structure (by ref)"))
  (if (`ActorComponent.ComponentHasTag` OtherComp "RightCalibration")
    (bind _output_get (set `self.RightHandInside` true))
    (`KismetSystemLibrary.PrintString` "Right Hand Entered" _output_get _output_get (struct :`R` 1.0 :`B` 0.051269 :`A` 1.0) 10.0)))

(event `self.RightTrigger.OnComponentEndOverlap`
  (params (OverlappedComponent :type "PrimitiveComponent Object Reference") (OtherActor :type "Actor Object Reference") (OtherComp :type "PrimitiveComponent Object Reference") (OtherBodyIndex :type Integer))
  (if (`ActorComponent.ComponentHasTag` OtherComp "RightCalibration")
    (bind _output_get (set `self.RightHandInside` false))
    (`KismetSystemLibrary.PrintString` "Right Hand Left" _output_get _output_get (struct :`R` 1.0 :`B` 0.051269 :`A` 1.0) 10.0)))

(fn `UserConstructionScript`)