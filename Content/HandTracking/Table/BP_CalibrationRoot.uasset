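; Calibration root actor for the hand-tracking table, anchoring the virtual table and the spawn points for its props.
; SetVirtualWorldVisible shows or hides the table and Props components without propagating to their children.
; SpawnProps prints a debug message, then spawns a chest at the centre point and GrabbablePolyhedra at the left and right points, each spawn gated on the previous one's validity.
; BeginPlay and the construction script are empty.
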(event `self.ReceiveBeginPlay`)

(event `SetVirtualWorldVisible`
  (params (Visible :type Boolean))
  (`SceneComponent.SetVisibility` (`self.VirtaulTable`) Visible false)
  (`SceneComponent.SetVisibility` (`self.Props`) Visible false))

(event `SpawnProps`
  (bind _returnvalue_location (`KismetMathLibrary.BreakTransform` (`SceneComponent.K2_GetComponentToWorld` (`self.CentreProp`))))
  (bind _returnvalue_location_2 (`KismetMathLibrary.BreakTransform` (`SceneComponent.K2_GetComponentToWorld` (`self.LeftProps`))))
  (bind _returnvalue_location_3 (`KismetMathLibrary.BreakTransform` (`SceneComponent.K2_GetComponentToWorld` (`self.RightPops`))))
  (`KismetSystemLibrary.PrintString` "SPAWN PROPS CALLED" true true (struct :`G` 0.66 :`B` 1.0 :`A` 1.0) 10.0)
  (bind _returnvalue (`|SpawnActorFromClass` "/Game/Assets/Chest/BP_New_Chest.BP_New_Chest_C" (`KismetMathLibrary.MakeTransform` _returnvalue_location (struct :`Yaw` 180.0)) "AlwaysSpawn" "MultiplyWithRoot" null null))
  (`/Engine/EditorBlueprintResources/StandardMacros.IsValid` _returnvalue
    (:`Is Valid`
      (bind _returnvalue_2 (`|SpawnActorFromClass` "/Game/SampleExamples/Objects/Props/StonePolyhedra/GrabbablePolyhedra.GrabbablePolyhedra_C" (`KismetMathLibrary.MakeTransform` _returnvalue_location_2 (struct :`Yaw` 180.0)) "AlwaysSpawn" "MultiplyWithRoot" null null))
      (`/Engine/EditorBlueprintResources/StandardMacros.IsValid` _returnvalue_2
        (:`Is Valid`
          (bind _returnvalue_3 (`|SpawnActorFromClass` "/Game/SampleExamples/Objects/Props/StonePolyhedra/GrabbablePolyhedra.GrabbablePolyhedra_C" (`KismetMathLibrary.MakeTransform` _returnvalue_location_3 (struct :`Yaw` 180.0)) "AlwaysSpawn" "MultiplyWithRoot" null null))
          (`/Engine/EditorBlueprintResources/StandardMacros.IsValid` _returnvalue_3))))))

(fn `UserConstructionScript`)