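; VR pawn for Meta Interaction SDK hand tracking that turns pinch grabs into calibration point signals.
; On BeginPlay, with an HMD enabled, it sets a local-floor tracking origin and adds the hand and controller-animation Enhanced Input mapping contexts.
; Left or right pinch reads joint 0 from that side's motion controller and broadcasts its position to every actor implementing BPI_Calibration.
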(event `self.ReceiveBeginPlay`
  (bind _returnvalue (pcsubsystem `EnhancedInputLocalPlayerSubsystem` (`GameplayStatics.GetPlayerController` 0)))
  ; Setting Tracking Space
  (if (`HeadMountedDisplayFunctionLibrary.IsHeadMountedDisplayEnabled`)
    (`HeadMountedDisplayFunctionLibrary.SetTrackingOrigin` "LocalFloor")
    ; Adding Input Mapping
    (`EnhancedInputSubsystemInterface.AddMappingContext` _returnvalue "/OculusInteraction/Inputs/IMC_IsdkHand.IMC_IsdkHand" 0 (struct))
    (`EnhancedInputSubsystemInterface.AddMappingContext` _returnvalue "/OculusInteraction/Inputs/IMC_IsdkControllerAnimation.IMC_IsdkControllerAnimation" 0 (struct))))

(event `GetHandCalibrationSignal`
  (params (IsLeftHand :type Boolean))
  (if IsLeftHand
    (bind (_bvaluefound _returnvalue) (`MotionControllerComponent.GetHandJointPosition` (`self.LeftMotionController`) 0))
    (bind _outactors (`GameplayStatics.GetAllActorsWithInterface` "/Game/HandTracking/Calibration/BPI_Calibration.BPI_Calibration_C"))
    (for _array_element _outactors
      (message `/Game/HandTracking/Calibration/BPI_Calibration.SendCalibrationPoint` _array_element _returnvalue))
    (else
      (bind (_bvaluefound_2 _returnvalue_2) (`MotionControllerComponent.GetHandJointPosition` (`self.RightMotionController`) 0))
      (bind _outactors_2 (`GameplayStatics.GetAllActorsWithInterface` "/Game/HandTracking/Calibration/BPI_Calibration.BPI_Calibration_C"))
      (for _array_element_2 _outactors_2
        (message `/Game/HandTracking/Calibration/BPI_Calibration.SendCalibrationPoint` _array_element_2 _returnvalue_2)))))

(event `EnhancedInput|/OculusInteraction/Inputs/IA_Left_HandPinchGrab`
  (params (ActionValue :type Boolean) (ElapsedSeconds :type "Float (double-precision)") (TriggeredSeconds :type "Float (double-precision)") (InputAction :type "InputAction Object Reference" :default "/OculusInteraction/Inputs/IA_Left_HandPinchGrab.IA_Left_HandPinchGrab"))
  (:`Triggered`
    (`self.GetHandCalibrationSignal` true)))

(event `EnhancedInput|/OculusInteraction/Inputs/IA_Right_HandPinchGrab`
  (params (ActionValue :type Boolean) (ElapsedSeconds :type "Float (double-precision)") (TriggeredSeconds :type "Float (double-precision)") (InputAction :type "InputAction Object Reference" :default "/OculusInteraction/Inputs/IA_Right_HandPinchGrab.IA_Right_HandPinchGrab"))
  (:`Triggered`
    (`self.GetHandCalibrationSignal` false)))

(fn `UserConstructionScript`)